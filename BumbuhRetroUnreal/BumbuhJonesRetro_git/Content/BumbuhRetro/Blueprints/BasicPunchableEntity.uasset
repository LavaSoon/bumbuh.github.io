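; Configurable punchable entity that the player destroys to grow stronger.
; While the player overlaps TriggerBox, Tick polls IsAttacking; a DoOnce and short Delay throttle hits, each raising PunchPower slightly and subtracting it from Health.
; Once Health drops below zero, it grants Reward as PunchPower, plays a sound, posts a message to the player's action text and destroys itself.
; The construction script applies mesh, material, scale and trigger overrides.
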(event OnComponentBeginOverlap(TriggerBox)
  (params (OtherActor :type Actor%20Object%20Reference) (OtherComp :type Primitive%20Component%20Object%20Reference) (OtherBodyIndex :type Integer) (bFromSweep :type Boolean) (SweepResult :type Hit%20Result%20Structure%20%28by%20ref%29))
  (if (Actor|ActorHasTag OtherActor "Player")
    (Variables|Default|SetisEntered? true)))

(event OnComponentEndOverlap(TriggerBox)
  (params (OtherActor :type Actor%20Object%20Reference) (OtherComp :type Primitive%20Component%20Object%20Reference) (OtherBodyIndex :type Integer))
  (Variables|Default|SetisEntered? false))

(event EventTick
  (params (DeltaSeconds :type Float%20%28single-precision%29))
  (if (>= (Variables|Default|GetHealth) 0.0)
    (if (Variables|Default|GetisEntered?)
      (bind _asthird_person_character (Utilities|Casting|CastToThirdPersonCharacter (Game|GetPlayerCharacter 0)))
      (if (Variables|/Game/ThirdPersonBP/Blueprints/ThirdPersonCharacter.ThirdPersonCharacter_C|GetisAttacking? _asthird_person_character)
        (Utilities|FlowControl|DoOnce false :!label _label
          (:Completed
            (Variables|/Game/ThirdPersonBP/Blueprints/ThirdPersonCharacter.ThirdPersonCharacter_C|SetPunchPower _asthird_person_character (+ (Variables|/Game/ThirdPersonBP/Blueprints/ThirdPersonCharacter.ThirdPersonCharacter_C|GetPunchPower _asthird_person_character) 0.025))
            (Class|GameplayStatics|PlaySoundAttached (Variables|Default|GetHitSound) (Variables|Default|GetCube))
            (Utilities|FlowControl|Delay 0.2)
            (Variables|Default|SetHealth (- (Variables|Default|GetHealth) (Variables|/Game/ThirdPersonBP/Blueprints/ThirdPersonCharacter.ThirdPersonCharacter_C|GetPunchPower _asthird_person_character)))
            (goto _label Reset)))))
    (else
      (bind _asthird_person_character_2 (Utilities|Casting|CastToThirdPersonCharacter (Game|GetPlayerCharacter 0)))
      (Variables|/Game/ThirdPersonBP/Blueprints/ThirdPersonCharacter.ThirdPersonCharacter_C|SetPunchPower _asthird_person_character_2 (+ (Variables|/Game/ThirdPersonBP/Blueprints/ThirdPersonCharacter.ThirdPersonCharacter_C|GetPunchPower _asthird_person_character_2) (Variables|Default|GetReward)))
      (Class|GameplayStatics|PlaySoundAttached (Variables|Default|GetDeathSound) (Variables|Default|GetCube))
      (Utilities|Array|Insert (Variables|/Game/ThirdPersonBP/Blueprints/ThirdPersonCharacter.ThirdPersonCharacter_C|GetCurrentActionText _asthird_person_character_2) (Utilities|String|Append (Utilities|String|Append "[BUMBUH destroys a " (Variables|Default|GetEntity%20Name)) "]"))
      (Actor|DestroyActor))))

(fn ConstructionScript
  (Components|StaticMesh|SetStaticMesh (Variables|Default|GetCube) (Variables|Default|GetStatic%20Mesh%20Replacement))
  (Transformation|SetActorScale3D (Math|Conversions|ToVector(Float) (Variables|Default|GetNew%20Mesh%20Scale)))
  (Transformation|SetRelativeScale3D (Variables|Default|GetTriggerBox) (Variables|Default|GetNew%20Trigger%20Scale))
  (Rendering|Material|SetMaterial (Variables|Default|GetCube) 0 (Variables|Default|GetNew%20Material))
  (Transformation|AddRelativeLocation (Variables|Default|GetTriggerBox) (Variables|Default|GetTrigger%20Location) false))